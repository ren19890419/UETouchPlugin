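; Player controller for touch input that shows a test touch widget and forwards finger events to Touch.
; BeginPlay creates BP_TastTouchWidget, adds it to the viewport, shows the cursor and sets Game and UI input mode focused on the widget.
; Press, release and move all call Touch.Touch with location and finger index.
; Only moves overwrite the location's Z with a constant; press and release pass it unchanged.
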(event `self.ReceiveBeginPlay`
  (bind _returnvalue (`|CreateWidget` "/UlTouch/BP_TastTouchWidget.BP_TastTouchWidget_C" self))
  (`UserWidget.AddToViewport` _returnvalue 0)
  (set `self.bShowMouseCursor` true)
  (`WidgetBlueprintLibrary.SetInputMode_GameAndUIEx` self _returnvalue "DoNotLock" false))

(event `InputTouch`
  (params (Location :type "Vector Structure") (FingerIndex :type "ETouchIndex Enum"))
  (bind _touch (`self.Touch`))
  (:`Pressed`
    (`TouchComponent.Touch` _touch Location FingerIndex))
  (:`Released`
    (`TouchComponent.Touch` _touch Location FingerIndex))
  (:`Moved`
    (`TouchComponent.Touch` _touch (`KismetMathLibrary.MakeVector` (.x Location) (.y Location) 2.0) FingerIndex)))

(fn `UserConstructionScript`)